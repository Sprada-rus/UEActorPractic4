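; BP_CUBE2 is an Actor, named as a cube, that shrinks each time another actor begins overlapping it.
; Each overlap reduces the stored Size variable by five percent, prints the new value on screen and applies it as the actor's 3D scale.
; The reduction compounds with no lower limit, and BeginPlay, Tick and the construction script add no logic of their own.
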(event `self.ReceiveActorBeginOverlap`
  (params (OtherActor :type "Actor Object Reference"))
  (bind _size (`self.Size`))
  (bind _returnvalue (- _size (* _size 0.05)))
  (cast `Actor` OtherActor)
  (`KismetSystemLibrary.PrintString` (`KismetStringLibrary.Conv_VectorToString` _returnvalue) true true (struct :`R` 0.075911 :`B` 1.0 :`A` 1.0) 5.0)
  (bind _output_get (set `self.Size` _returnvalue))
  (`self.SetActorScale3D` _output_get))

(fn `UserConstructionScript`
  (`parent.UserConstructionScript`))