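; BP_Cube is an actor that destroys itself after a set number of overlaps.
; Each overlap with any actor increments Count and compares it to MaxCount.
; When the two are equal it calls DestroyActor; otherwise it prints the current count on screen as debug text.
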(event `self.ReceiveActorBeginOverlap`
  (params (OtherActor :type "Actor Object Reference"))
  (cast `Actor` OtherActor)
  (bind _result (`/Engine/EditorBlueprintResources/StandardMacros.IncrementInt` (`self.count`))
    (:`  `
      (bind _output_get (set `self.count` _result))
      (if (== _output_get (`self.maxCount`))
        (`self.K2_DestroyActor`)
        (else
          (`KismetSystemLibrary.PrintString` (`KismetStringLibrary.Conv_IntToString` (`self.count`)) true false (struct :`R` 1.0 :`G` 0.070318 :`A` 1.0) 5.0))))))

(fn `UserConstructionScript`)